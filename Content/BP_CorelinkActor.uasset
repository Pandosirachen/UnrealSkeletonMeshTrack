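; Actor that replays streamed Corelink pose data onto test balls and a character skeleton.
; At a capped framerate, Tick parses the CorelinkVar string into seven-float groups of position plus quaternion.
; Each group teleports a ball from the GameMode's list, with axes remapped and scaled.
; UpdateMesh feeds scaled positions and converted rotations to the B_Corelink AnimInstance; per-bone rotation corrections exist but are disconnected.
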(event `Set up spheres`
  (bind _asgm_corelink_sphere_test (cast `/Game/GM_CorelinkSphereTest` (`GameplayStatics.GetGameMode`)))
  (set `self.Testballs` (`/Game/GM_CorelinkSphereTest.TestActors` _asgm_corelink_sphere_test))
  (set `self.IsTestballSetup` true))

(event `self.ReceiveTick`
  (params (DeltaSeconds :type "Float (single-precision)"))
  (bind _returnvalue (`KismetStringLibrary.ParseIntoArray` (`self.StringTest`)))
  ;[1 1 1] Timer
  (bind _output_get (set `self.Timer` (+ DeltaSeconds (`self.Timer`))))
  (if (> _output_get (/ 1.0 (`self.framerate`)))
    (set `self.Timer` 0.0)
    (set `self.StringTest` (`self.CorelinkVar`))
    ;[1 1 1] Corelink Test print
    (set `self.String Array` _returnvalue)
    (for _index (range (/ (`KismetArrayLibrary.Array_Length` _returnvalue) 7))
      (bind (_newparam _newparam1 _newparam2 _rx _ry _rz) (`self.Get Corelink Vectors` _returnvalue _index))
      (`self.Teleport Test Ball` _newparam _newparam1 _newparam2 _index _rx _ry _rz)
      (`self.UpdateMesh`))))

(event `Spawn Testball`
  (params (X :type String) (Y :type String) (Z :type String))
  (bind _scale (`self.Scale`))
  ;[1 1 1] Spawn Testball
  (bind _vector (`self.Combine String To Vector` X Y Z))
  (`|SpawnActorFromClass` "/Game/BP_TestActor.BP_TestActor_C" (`KismetMathLibrary.MakeTransform` (`KismetMathLibrary.MakeVector` (* (.x _vector) _scale) (* (.y _vector) _scale) (* (.z _vector) _scale)) (struct) (5.0 5.0 5.0)) "Undefined" "OverrideRootScale" null (`self.Test Ball Alive Time`) null))

(event `Teleport Test Ball`
  (params (X :type String) (Y :type String) (Z :type String) (index :type Integer) (RX :type String) (RY :type String) (RZ :type String))
  (bind _scale (`self.Scale`))
  ;[1 1 1] Teleport test ball
  (bind _vector (`self.Combine String To Vector` RX RY RZ))
  (bind _vector_2 (`self.Combine String To Vector` X Y Z))
  (`self.K2_TeleportTo` (`|GetArrayItem` (`self.Testballs`) index) (`KismetMathLibrary.MakeVector` (* (.z _vector_2) _scale) (* (.x _vector_2) _scale) (* (.y _vector_2) _scale)) (`KismetMathLibrary.MakeRotator` (* (.x _vector) 1.0) (* (.y _vector) 1.0) (* (.z _vector) 1.0))))

(event `UpdateMesh`
  ;[1 1 1] Mesh Test
  (bind _asb_corelink (cast `/Game/Blueprints/B_Corelink` (`SkeletalMeshComponent.GetAnimInstance` (`self.Character`))))
  (bind (_pos_arr _rot_arr) (`self.StringArray toVectorArray` (`self.String Array`)))
  (set `/Game/Blueprints/B_Corelink.PositionList` _pos_arr _asb_corelink)
  (set `/Game/Blueprints/B_Corelink.RotationList` _rot_arr _asb_corelink))

(fn `Combine String To Vector`
  (params (String1 :type String) (String2 :type String) (String3 :type String))
  (returns (Vector :type "Vector Structure"))
  (return (`KismetMathLibrary.MakeVector` (`KismetStringLibrary.Conv_StringToDouble` String1) (`KismetStringLibrary.Conv_StringToDouble` String2) (`KismetStringLibrary.Conv_StringToDouble` String3))))

(fn `Get Corelink Vectors`
  (params (FloatStringArray :type "Array of String") (Index :type Integer))
  (returns (NewParam :type String) (NewParam1 :type String) (NewParam2 :type String) (RX :type String) (RY :type String) (RZ :type String))
  (locals (Quaternian :type "Quat Structure"))
  (bind _returnvalue (* Index 7))
  (bind _output_get (set `local.Quaternian` (`KismetMathLibrary.MakeQuat` (`KismetStringLibrary.Conv_StringToDouble` (`|GetArrayItem` FloatStringArray (+ _returnvalue 3))) (`KismetStringLibrary.Conv_StringToDouble` (`|GetArrayItem` FloatStringArray (+ _returnvalue 4))) (`KismetStringLibrary.Conv_StringToDouble` (`|GetArrayItem` FloatStringArray (+ _returnvalue 5))) (`KismetStringLibrary.Conv_StringToDouble` (`|GetArrayItem` FloatStringArray (+ _returnvalue 6))))))
  (bind (_returnvalue_roll _returnvalue_pitch _returnvalue_yaw) (`KismetMathLibrary.BreakRotator` (`KismetMathLibrary.Quat_Rotator` _output_get)))
  (return (`|GetArrayItem` FloatStringArray _returnvalue) (`|GetArrayItem` FloatStringArray (+ _returnvalue 1)) (`|GetArrayItem` FloatStringArray (+ _returnvalue 2)) (`KismetStringLibrary.Conv_DoubleToString` _returnvalue_roll) (`KismetStringLibrary.Conv_DoubleToString` _returnvalue_pitch) (`KismetStringLibrary.Conv_DoubleToString` _returnvalue_yaw)))

(fn `Print Corelink Vector`
  (params (X :type String) (Y :type String) (Z :type String) (Duration :type "Float (double-precision)"))
  (`KismetSystemLibrary.PrintString` (`KismetStringLibrary.Concat_StrStr` (`KismetStringLibrary.Concat_StrStr` (`KismetStringLibrary.Concat_StrStr` (`KismetStringLibrary.Concat_StrStr` X ",") Y) ",") Z) true true (struct :`G` 0.66 :`B` 1.0 :`A` 1.0) Duration))

(fn `StringArray toVectorArray`
  (params (StringArr :type "Array of String"))
  (returns (`Pos Arr` :type "Array of Vector Structure") (`Rot Arr` :type "Array of Rotator Structure"))
  (locals (TempArr :type "Array of Vector Structure") (TempRot :type "Array of Rotator Structure"))
  (bind _temparr (`local.TempArr`))
  (bind _temprot (`local.TempRot`))
  (for _index (range (+ (/ (`KismetArrayLibrary.Array_Length` StringArr) 7) 1))
    (bind _returnvalue (* _index 7))
    (bind _vector (`self.Combine String To Vector` (`|GetArrayItem` StringArr (+ _returnvalue 0)) (`|GetArrayItem` StringArr (+ _returnvalue 1)) (`|GetArrayItem` StringArr (+ _returnvalue 2))))
    (`KismetArrayLibrary.Array_Add` _temparr (* _vector (`self.Mesh Scale`)))
    (`KismetArrayLibrary.Array_Add` _temprot (`KismetMathLibrary.Quat_Rotator` (`KismetMathLibrary.MakeQuat` (`KismetStringLibrary.Conv_StringToDouble` (`|GetArrayItem` StringArr (+ _returnvalue 3))) (`KismetStringLibrary.Conv_StringToDouble` (`|GetArrayItem` StringArr (+ _returnvalue 4))) (`KismetStringLibrary.Conv_StringToDouble` (`|GetArrayItem` StringArr (+ _returnvalue 5))) (`KismetStringLibrary.Conv_StringToDouble` (`|GetArrayItem` StringArr (+ _returnvalue 6)))))))
  (return _temparr _temprot))

(fn `UserConstructionScript`)